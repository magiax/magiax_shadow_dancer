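; AI controller for the Chemist boss's ghost, which travels to a respawn point so the boss can reincarnate.
; MoveToRespawn waits briefly, then issues AIMoveTo toward the target, retrying if the pawn's horizontal velocity is near zero right after the move starts.
; On arrival, it casts the pawn to BP_Boss_Chemist_Ghost and calls Reincornation on its parent reference.
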(event `MoveToRespawn`
  (params (TargetLocation :type "Vector Structure"))
  (`KismetSystemLibrary.Delay` 1.0 :!label _label)
  (`|AIMoveTo` null TargetLocation null 100.0
    (:`then`
      (if (< (`KismetMathLibrary.VSizeXY` (`self.GetVelocity` (`self.K2_GetPawn`))) 2.0)
        (goto _label)))
    (:`OnSuccess`
      (bind _asbp_boss_chemist_ghost (cast `/Game/XYZ_GD_Project/Core/Enemys/Boss_Chemist/BP_Boss_Chemist_Ghost` (`self.K2_GetPawn`)))
      (`/Game/XYZ_GD_Project/Core/Enemys/BP_BossChemist.Reincornation` (`/Game/XYZ_GD_Project/Core/Enemys/Boss_Chemist/BP_Boss_Chemist_Ghost.refParrent` _asbp_boss_chemist_ghost)))))

(fn `UserConstructionScript`)