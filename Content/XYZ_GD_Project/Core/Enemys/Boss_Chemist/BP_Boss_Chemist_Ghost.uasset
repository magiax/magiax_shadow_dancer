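; Ghost minion of the Chemist boss that travels to a given target through its AI controller, moving faster in higher phases.
; While the medallion is exposed, one BP_DamageAll hit swaps it for a shield, plays audio and notifies the parent; Restart re-exposes it.
; Gas and shield particle collisions apply tiny-radius damage that affects only the player.
; preDestroy hides the visuals and ends gas trails before a delayed destroy.
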(event `SetParams`
  (params (refParrent :type "/Game/XYZ_GD_Project/Core/Enemys/BP_BossChemist Object Reference") (Target :type "Vector Structure") (iFaza :type Integer))
  ;[1 1 1] Ref Parrent
  (set `self.refParrent` refParrent)
  (bind _output_get (set `self.Target` Target))
  (bind _asbp_ai_boss_ghost (cast `/Game/XYZ_GD_Project/Core/Enemys/Boss_Chemist/AI/BP_AI_Boss_Ghost` (`AIBlueprintHelperLibrary.GetAIController` (`self.GetOwner`))))
  (`/Game/XYZ_GD_Project/Core/Enemys/Boss_Chemist/AI/BP_AI_Boss_Ghost.MoveToRespawn` _asbp_ai_boss_ghost _output_get)
  (set `CharacterMovementComponent.MaxWalkSpeed` (+ (* iFaza 50.0) 150.0) (`self.CharacterMovement`)))

(event `self.ReceiveBeginPlay`
  ;[1 1 1] Constructor
  (`self.Restart`)
  (`ActorComponent.Activate` (`self.NavigationInvoker`) true))

(event `Restart`
  ;[1 1 1] Restart
  (`SceneComponent.SetVisibility` (`self.PS_Shield`) false true)
  (`SceneComponent.SetVisibility` (`self.SM_Medalon`) true true)
  (set `self.bIsOpenDamage` true))

(event `preDestroy`
  ;[1 1 1] PreDestroy
  (`SceneComponent.SetVisibility` (`self.SM_Medalon`) false true)
  (`SceneComponent.SetVisibility` (`self.PS_Shield`) false true)
  (`ParticleSystemComponent.EndTrails` (`self.PS_Gas`))
  (set `self.bIsOpenDamage` false)
  (`KismetSystemLibrary.Delay` 5.0)
  (`self.K2_DestroyActor`))

(event `ShieldActive`
  ;[1 1 1] Shield Active
  (`SceneComponent.SetVisibility` (`self.PS_Shield`) true true)
  (`SceneComponent.SetVisibility` (`self.SM_Medalon`) false true))

(event `self.ReceiveAnyDamage`
  (params (Damage :type "Float (single-precision)") (DamageType :type "DamageType Object Reference") (InstigatedBy :type "Controller Object Reference") (DamageCauser :type "Actor Object Reference"))
  (bind _refparrent (`self.refParrent`))
  ;[1 1 1] Any Damage
  (if (and (== (`GameplayStatics.GetObjectClass` DamageType) "/Game/XYZ_GD_Project/Weapons/BP_DamageAll.BP_DamageAll_C") (`self.bIsOpenDamage`) true)
    (set `self.bIsOpenDamage` false)
    (`self.ShieldActive`)
    (`AudioComponent.Play` (`self.AudioGhost`) 0.0)
    (`KismetSystemLibrary.Delay` 0.2)
    (`AudioComponent.Play` (`self.AudioGhostVoice`) 0.0)
    (`/Engine/EditorBlueprintResources/StandardMacros.IsValid` _refparrent
      (:`Is Valid`
        (`/Game/XYZ_GD_Project/Core/Enemys/BP_BossChemist.ActiveGhostDamage` _refparrent)))))

(event `self.PS_Gas.OnParticleCollide`
  (params (EventName :type Name) (EmitterTime :type "Float (single-precision)") (ParticleTime :type Integer) (Location :type "Vector Structure") (Velocity :type "Vector Structure") (Direction :type "Vector Structure") (Normal :type "Vector Structure") (BoneName :type Name) (PhysMat :type "PhysicalMaterial Object Reference"))
  (bind _fdamage (`self.fDamage`))
  ;[1 0.2499 0.2599] Gas Damage
  (`GameplayStatics.ApplyRadialDamageWithFalloff` :`BaseDamage` _fdamage :`MinimumDamage` _fdamage :`Origin` Location :`DamageInnerRadius` 1.0 :`DamageOuterRadius` 1.0 :`DamageFalloff` 2.0 :`DamageTypeClass` "/Game/XYZ_GD_Project/Weapons/BP_DamageOnlyPlayer.BP_DamageOnlyPlayer_C" :`DamageCauser` null :`InstigatedByController` null))

(event `self.PS_Shield.OnParticleCollide`
  (params (EventName :type Name) (EmitterTime :type "Float (single-precision)") (ParticleTime :type Integer) (Location :type "Vector Structure") (Velocity :type "Vector Structure") (Direction :type "Vector Structure") (Normal :type "Vector Structure") (BoneName :type Name) (PhysMat :type "PhysicalMaterial Object Reference"))
  (bind _fdamage (`self.fDamage`))
  ;[1 0.2499 0.2599] Gas Damage
  (`GameplayStatics.ApplyRadialDamageWithFalloff` :`BaseDamage` _fdamage :`MinimumDamage` _fdamage :`Origin` Location :`DamageInnerRadius` 1.0 :`DamageOuterRadius` 1.0 :`DamageFalloff` 2.0 :`DamageTypeClass` "/Game/XYZ_GD_Project/Weapons/BP_DamageOnlyPlayer.BP_DamageOnlyPlayer_C" :`DamageCauser` null :`InstigatedByController` null))

(fn `UserConstructionScript`)