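; One body of the Chemist boss, with its health and phase bar, medallion, voice and gas attack effects.
; Life toggles switch collision, medallion and UI; death starts posthumous gas after a delay and notifies the parent reference.
; BP_DamageAll hits on a living body are forwarded to the owning BP_AI_Boss_Chemist.
; Wave attacks reuse pre-placed particle emitters, and gas particle collisions apply player-only radial damage.
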(event `SetLife`
  (params (bLife :type Boolean))
  (bind _bislife (`self.bIsLife`))
  ;[1 1 1] Get/SetFromAIController
  (if bLife
    (if (not _bislife)
      (`self.BPLife`))
    (elif _bislife
      (`self.BPDeath`))))

(event `SetRefParrent`
  (params (refParrent :type "/Game/XYZ_GD_Project/Core/Enemys/BP_BossChemist Object Reference"))
  ;[0.474 0.3174 0.1437] SetRefParrent
  (bind _output_get (set `self.refParrent` refParrent))
  (`self.PlayVoice` _output_get))

(event `VisibilityMedal`
  (params (bView :type Boolean))
  ;[1 1 1] Visibility Medal
  (`SceneComponent.SetVisibility` (`self.SM_Medalon`) bView bView))

(event `SetActualHealt`
  (params (fMaxHealt :type "Float (double-precision)") (fHealt :type "Float (double-precision)"))
  ;[1 1 1] Get/SetFromAIController
  (set `self.MaxHealt` fMaxHealt)
  (set `self.Healt` fHealt)
  (`self.SetShowUI`))

(event `BPLife`
  ;[0.0102 0.9801 1] Life
  (set `self.Healt` (`self.MaxHealt`))
  (set `self.bIsLife` true)
  (`SceneComponent.SetVisibility` (`self.HealtUI`) true false)
  (`self.Gas Clapons` false)
  (`self.SetCollision` "QueryAndPhysics")
  (`self.VisibilityMedal` true))

(event `SetShowUI`
  ;[1 1 1] Refrash Data UI
  (bind _asumg_npc_life (cast `/Game/XYZ_GD_Project/UMG/UMG_NPC_Life` (`WidgetComponent.GetUserWidgetObject` (`self.HealtUI`))))
  (`/Game/XYZ_GD_Project/UMG/UMG_NPC_Life.RefrashLifeBar` _asumg_npc_life (`self.Healt`) (`self.MaxHealt`)))

(event `SetFaza`
  (params (iFaza :type Integer))
  ;[1 1 1] Refrash Faza UI
  (bind _asumg_npc_life (cast `/Game/XYZ_GD_Project/UMG/UMG_NPC_Life` (`WidgetComponent.GetUserWidgetObject` (`self.HealtUI`))))
  (`/Game/XYZ_GD_Project/UMG/UMG_NPC_Life.RefrashAgression` _asumg_npc_life (`KismetMathLibrary.Conv_IntToDouble` iFaza) 1.0 4.0))

(event `BPDeath`
  (bind _refparrent (`self.refParrent`))
  ;[0 0.6315 1] Death
  (`AudioComponent.Stop` (`self.Gas`))
  (set `self.bIsLife` false)
  (`SceneComponent.SetVisibility` (`self.HealtUI`) false false)
  (`KismetSystemLibrary.Delay` 3.0)
  (`self.Gas Clapons` true)
  (`self.SetCollision` "NoCollision")
  (`self.VisibilityMedal` false)
  (`/Engine/EditorBlueprintResources/StandardMacros.IsValid` _refparrent
    (:`Is Valid`
      (`/Game/XYZ_GD_Project/Core/Enemys/BP_BossChemist.ActiveBodyDeath` _refparrent))))

(event `self.PS_Gas_Wave.OnParticleCollide`
  (params (EventName :type Name) (EmitterTime :type "Float (single-precision)") (ParticleTime :type Integer) (Location :type "Vector Structure") (Velocity :type "Vector Structure") (Direction :type "Vector Structure") (Normal :type "Vector Structure") (BoneName :type Name) (PhysMat :type "PhysicalMaterial Object Reference"))
  (bind _fgasdamage (`self.fGasDamage`))
  ;[0.1036 1 0.2361] Posthumous Damage Gas
  (`GameplayStatics.ApplyRadialDamageWithFalloff` :`BaseDamage` _fgasdamage :`MinimumDamage` _fgasdamage :`Origin` Location :`DamageOuterRadius` 5.0 :`DamageTypeClass` "/Game/XYZ_GD_Project/Weapons/BP_DamageOnlyPlayer.BP_DamageOnlyPlayer_C" :`DamageCauser` null :`InstigatedByController` null))

(event `self.PS_Posthumous_head.OnParticleCollide`
  (params (EventName :type Name) (EmitterTime :type "Float (single-precision)") (ParticleTime :type Integer) (Location :type "Vector Structure") (Velocity :type "Vector Structure") (Direction :type "Vector Structure") (Normal :type "Vector Structure") (BoneName :type Name) (PhysMat :type "PhysicalMaterial Object Reference"))
  (bind _fgasdamage (`self.fGasDamage`))
  ;[0.1036 1 0.2361] Posthumous Damage Gas
  (`GameplayStatics.ApplyRadialDamageWithFalloff` :`BaseDamage` _fgasdamage :`MinimumDamage` _fgasdamage :`Origin` Location :`DamageOuterRadius` 5.0 :`DamageTypeClass` "/Game/XYZ_GD_Project/Weapons/BP_DamageOnlyPlayer.BP_DamageOnlyPlayer_C" :`DamageCauser` null :`InstigatedByController` null))

(event `self.ReceiveAnyDamage`
  (params (Damage :type "Float (single-precision)") (DamageType :type "DamageType Object Reference") (InstigatedBy :type "Controller Object Reference") (DamageCauser :type "Actor Object Reference"))
  ;[1 1 1] Translite Damage
  (if (and (== (`GameplayStatics.GetObjectClass` DamageType) "/Game/XYZ_GD_Project/Weapons/BP_DamageAll.BP_DamageAll_C") (`self.bIsLife`) true)
    (bind _asbp_ai_boss_chemist (cast `/Game/XYZ_GD_Project/Core/Enemys/Boss_Chemist/AI/BP_AI_Boss_Chemist` (`self.GetOwner`)))
    (`/Game/XYZ_GD_Project/Core/Enemys/Boss_Chemist/AI/BP_AI_Boss_Chemist.SetDamage` _asbp_ai_boss_chemist Damage)))

(event `self.PS_Posthumous_body_up.OnParticleCollide`
  (params (EventName :type Name) (EmitterTime :type "Float (single-precision)") (ParticleTime :type Integer) (Location :type "Vector Structure") (Velocity :type "Vector Structure") (Direction :type "Vector Structure") (Normal :type "Vector Structure") (BoneName :type Name) (PhysMat :type "PhysicalMaterial Object Reference"))
  (bind _fgasdamage (`self.fGasDamage`))
  ;[0.1036 1 0.2361] Posthumous Damage Gas
  (`GameplayStatics.ApplyRadialDamageWithFalloff` :`BaseDamage` _fgasdamage :`MinimumDamage` _fgasdamage :`Origin` Location :`DamageOuterRadius` 5.0 :`DamageTypeClass` "/Game/XYZ_GD_Project/Weapons/BP_DamageOnlyPlayer.BP_DamageOnlyPlayer_C" :`DamageCauser` null :`InstigatedByController` null))

(event `SpawnGas`
  (params (iType :type Integer) (fDeltaZ :type "Float (double-precision)"))
  (bind _output (`|GetArrayItem` (`self.PS_Array_Gas`) (`self.iIndexGas`)))
  ;[1 1 1] Wave attack
  (`ParticleSystemComponent.SetTemplate` _output (`|GetArrayItem` (`self.AllGas`) iType))
  (`SceneComponent.K2_SetWorldLocation` _output (`KismetMathLibrary.MakeVector` (.x (.location (`SceneComponent.K2_GetComponentToWorld` (`self.Mesh`)))) (.y (.location (`SceneComponent.K2_GetComponentToWorld` (`self.Mesh`)))) (+ (.z (.location (`SceneComponent.K2_GetComponentToWorld` (`self.Mesh`)))) fDeltaZ)) false false)
  (`ParticleSystemComponent.BeginTrails` _output "None" "None" "ETrailWidthMode_FromCentre" 0.0)
  (if (>= (+ (`self.iIndexGas`) 1) (`KismetArrayLibrary.Array_Length` (`self.PS_Array_Gas`)))
    (set `self.iIndexGas` 0)))

(event `self.PS_Gas_Wave_1.OnParticleCollide`
  (params (EventName :type Name) (EmitterTime :type "Float (single-precision)") (ParticleTime :type Integer) (Location :type "Vector Structure") (Velocity :type "Vector Structure") (Direction :type "Vector Structure") (Normal :type "Vector Structure") (BoneName :type Name) (PhysMat :type "PhysicalMaterial Object Reference"))
  (bind _fgasdamage (`self.fGasDamage`))
  ;[0.1036 1 0.2361] Posthumous Damage Gas
  (`GameplayStatics.ApplyRadialDamageWithFalloff` :`BaseDamage` _fgasdamage :`MinimumDamage` _fgasdamage :`Origin` Location :`DamageOuterRadius` 5.0 :`DamageTypeClass` "/Game/XYZ_GD_Project/Weapons/BP_DamageOnlyPlayer.BP_DamageOnlyPlayer_C" :`DamageCauser` null :`InstigatedByController` null))

(event `self.PS_Posthumous_body_down.OnParticleCollide`
  (params (EventName :type Name) (EmitterTime :type "Float (single-precision)") (ParticleTime :type Integer) (Location :type "Vector Structure") (Velocity :type "Vector Structure") (Direction :type "Vector Structure") (Normal :type "Vector Structure") (BoneName :type Name) (PhysMat :type "PhysicalMaterial Object Reference"))
  (bind _fgasdamage (`self.fGasDamage`))
  ;[0.1036 1 0.2361] Posthumous Damage Gas
  (`GameplayStatics.ApplyRadialDamageWithFalloff` :`BaseDamage` _fgasdamage :`MinimumDamage` _fgasdamage :`Origin` Location :`DamageOuterRadius` 5.0 :`DamageTypeClass` "/Game/XYZ_GD_Project/Weapons/BP_DamageOnlyPlayer.BP_DamageOnlyPlayer_C" :`DamageCauser` null :`InstigatedByController` null))

(event `self.PS_Gas_Wave_2.OnParticleCollide`
  (params (EventName :type Name) (EmitterTime :type "Float (single-precision)") (ParticleTime :type Integer) (Location :type "Vector Structure") (Velocity :type "Vector Structure") (Direction :type "Vector Structure") (Normal :type "Vector Structure") (BoneName :type Name) (PhysMat :type "PhysicalMaterial Object Reference"))
  (bind _fgasdamage (`self.fGasDamage`))
  ;[0.1036 1 0.2361] Posthumous Damage Gas
  (`GameplayStatics.ApplyRadialDamageWithFalloff` :`BaseDamage` _fgasdamage :`MinimumDamage` _fgasdamage :`Origin` Location :`DamageOuterRadius` 5.0 :`DamageTypeClass` "/Game/XYZ_GD_Project/Weapons/BP_DamageOnlyPlayer.BP_DamageOnlyPlayer_C" :`DamageCauser` null :`InstigatedByController` null))

(event `self.ReceiveBeginPlay`
  (bind _ps_array_gas (`self.PS_Array_Gas`))
  ;[1 1 1] Gas pregen
  (`KismetArrayLibrary.Array_Add` _ps_array_gas (`self.PS_Gas_Wave`))
  (`KismetArrayLibrary.Array_Add` _ps_array_gas (`self.PS_Gas_Wave_1`))
  (`KismetArrayLibrary.Array_Add` _ps_array_gas (`self.PS_Gas_Wave_2`)))

(fn `Gas Clapons`
  (params (bIsActive :type Boolean))
  (bind _ps_posthumous_body_up (`self.PS_Posthumous_body_up`))
  (bind _ps_posthumous_body_down (`self.PS_Posthumous_body_down`))
  (bind _ps_posthumous_head (`self.PS_Posthumous_head`))
  (`ParticleSystemComponent.SetTemplate` (`self.PS_Posthumous_head`) "/Game/XYZ_GD_Project/Weapons/ParticleSystem/Gas/PS_Gas_Posthumous.PS_Gas_Posthumous")
  (`ParticleSystemComponent.SetTemplate` (`self.PS_Posthumous_body_up`) "/Game/XYZ_GD_Project/Weapons/ParticleSystem/Gas/PS_Gas_Posthumous.PS_Gas_Posthumous")
  (`ParticleSystemComponent.SetTemplate` (`self.PS_Posthumous_body_down`) "/Game/XYZ_GD_Project/Weapons/ParticleSystem/Gas/PS_Gas_Posthumous.PS_Gas_Posthumous")
  (if bIsActive
    (`ParticleSystemComponent.BeginTrails` _ps_posthumous_head "None" "None" "ETrailWidthMode_FromCentre" 0.0)
    (`ParticleSystemComponent.BeginTrails` _ps_posthumous_body_up "None" "None" "ETrailWidthMode_FromCentre" 0.0)
    (`ParticleSystemComponent.BeginTrails` _ps_posthumous_body_down "None" "None" "ETrailWidthMode_FromCentre" 0.0)
    (else
      (`ParticleSystemComponent.EndTrails` _ps_posthumous_head)
      (`ParticleSystemComponent.EndTrails` _ps_posthumous_body_up)
      (`ParticleSystemComponent.EndTrails` _ps_posthumous_body_down)))
  (return))

(fn `PlayGasAttack`
  (params (iSound :type Integer))
  (bind _gas (`self.Gas`))
  (`AudioComponent.SetSound` _gas (`|GetArrayItem` (`self.AttackGas`) iSound))
  (`AudioComponent.Play` _gas 0.0)
  (return))

(fn `PlayVoiceAttack`
  (params (iFaza :type Integer) (bTeleport :type Boolean))
  (bind _voice (`self.Voice`))
  (if bTeleport
    (`AudioComponent.SetSound` _voice "/Game/XYZ_GD_Project/Core/Enemys/Boss_Chemist/Voice/Body/Boss_Teleport_Cue.Boss_Teleport_Cue")
    (else
      (`AudioComponent.SetSound` _voice (`|GetArrayItem` (`self.AttackCue`) iFaza))))
  (`AudioComponent.Play` _voice 0.0)
  (return))

(fn `UserConstructionScript`)