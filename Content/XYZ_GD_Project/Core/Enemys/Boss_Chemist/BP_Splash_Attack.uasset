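; BP_Splash_Attack is a Chemist boss attack that creates a damaging gas splash, driven by particle collisions.
; The first ray particle collision starts the splash trails and Gas playback, then ends the trails after a set lifetime and destroys the actor following a short delay.
; Each splash particle collision applies small-radius radial damage with equal base and minimum values, using a player-only damage type.
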(event `self.PS_Ray.OnParticleCollide`
  (params (EventName :type Name) (EmitterTime :type "Float (single-precision)") (ParticleTime :type Integer) (Location :type "Vector Structure") (Velocity :type "Vector Structure") (Direction :type "Vector Structure") (Normal :type "Vector Structure") (BoneName :type Name) (PhysMat :type "PhysicalMaterial Object Reference"))
  (if (not (`self.bStartSplash`))
    (set `self.bStartSplash` true)
    (`ParticleSystemComponent.BeginTrails` (`self.PS_Splash`) "None" "None" "ETrailWidthMode_FromCentre" 0.0)
    (`AudioComponent.Play` (`self.Gas`) 0.0)
    (`KismetSystemLibrary.Delay` (`self.fLife`))
    (`ParticleSystemComponent.EndTrails` (`self.PS_Splash`))
    (`KismetSystemLibrary.Delay` 3.0)
    (`self.K2_DestroyActor`)))

(event `self.PS_Splash.OnParticleCollide`
  (params (EventName :type Name) (EmitterTime :type "Float (single-precision)") (ParticleTime :type Integer) (Location :type "Vector Structure") (Velocity :type "Vector Structure") (Direction :type "Vector Structure") (Normal :type "Vector Structure") (BoneName :type Name) (PhysMat :type "PhysicalMaterial Object Reference"))
  (bind _fgasdamage (`self.fGasDamage`))
  (`GameplayStatics.ApplyRadialDamageWithFalloff` :`BaseDamage` _fgasdamage :`MinimumDamage` _fgasdamage :`Origin` Location :`DamageOuterRadius` 5.0 :`DamageTypeClass` "/Game/XYZ_GD_Project/Weapons/BP_DamageOnlyPlayer.BP_DamageOnlyPlayer_C" :`DamageCauser` null :`InstigatedByController` null))

(fn `UserConstructionScript`)