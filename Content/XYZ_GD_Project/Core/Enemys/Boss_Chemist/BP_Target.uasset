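; BP_Target is a short-lived target marker actor for the Chemist boss that shrinks over its lifetime, then destroys itself.
; BeginPlay sets remaining life to the maximum and starts a fast looping timer.
; Each tick of that timer scales the Target component by the remaining life ratio plus a fixed offset and decrements life, clearing the timer and destroying the actor once it runs out.
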(event `self.ReceiveBeginPlay`
  (set `self.fLife` (`self.fMaxLife`))
  (bind _returnvalue (`KismetSystemLibrary.K2_SetTimerDelegate` (delegate `TargetLife`) 0.01 true))
  (set `self.Timer` _returnvalue))

(event `TargetLife`
  (bind _returnvalue (+ (/ (`self.fLife`) (`self.fMaxLife`)) 0.5))
  (if (> (`self.fLife`) 0.0)
    (`SceneComponent.SetWorldScale3D` (`self.Target`) (`KismetMathLibrary.MakeVector` _returnvalue _returnvalue _returnvalue))
    (set `self.fLife` (- (`self.fLife`) 0.01))
    (else
      (`KismetSystemLibrary.K2_ClearAndInvalidateTimerHandle` (`self.Timer`))
      (`self.K2_DestroyActor`))))

(fn `UserConstructionScript`)