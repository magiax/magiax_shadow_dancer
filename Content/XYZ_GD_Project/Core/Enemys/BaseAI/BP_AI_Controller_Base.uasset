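; Base AI controller for enemy NPCs, owning health, aggression, stun and life state.
; An init event pushes stats to the BP_NPC_Base pawn, reads patrol points and starts a timer decaying aggression, which updates the Blackboard SelfState against an attack threshold.
; Damage adds aggression, targets the player's location, plays a hurt sound and applies timed stun.
; Death stops the decay, unpossesses and calls the player's SetPitchGame.
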(event `self.ReceivePossess`
  (params (PossessedPawn :type "Pawn Object Reference"))
  ;[1 1 1] Refs
)

(event `RefrashBaseParems`
  ;[1 1 1] RefrashFromChaild
  (`BlackboardComponent.SetValueAsEnum` (`self.Blackboard`) "SelfState" 0)
  (`self.Dransfer Data Life BaseClass`)
  (`self.Dransfer Data Heals BaseClass`)
  (bind _asbp_npc_base (cast `/Game/XYZ_GD_Project/Core/Enemys/BP_NPC_Base` (`self.K2_GetPawn`)))
  (bind (_points _bispatrol) (`/Game/XYZ_GD_Project/Core/Enemys/BP_NPC_Base.GetPatrolPoints` _asbp_npc_base))
  (set `self.PatrolPoints` _points)
  (`BlackboardComponent.SetValueAsEnum` (`self.Blackboard`) "SelfState" 5)
  ;[0.5167 1 0.4638] DecreaseInAggression
  (bind _returnvalue (`KismetSystemLibrary.K2_SetTimerDelegate` (delegate `DecreaseInAggression`) 1.0 (`self.IsLife`)))
  (set `self.TimerDecreaseInAggression` _returnvalue))

(event `DecreaseInAggression`
  (bind _fagression (`self.fAgression`))
  ;[0.5167 1 0.4638] DecreaseInAggression
  (if (> _fagression 0.0)
    (bind _result (`/Engine/EditorBlueprintResources/StandardMacros.DecrementFloat` _fagression)
      (:`  `
        (`BlackboardComponent.SetValueAsFloat` (`AIBlueprintHelperLibrary.GetBlackboard` null) "fAgressive" _result)
        (`self.AgressionStatus`)
        (bind _asbp_npc_base (cast `/Game/XYZ_GD_Project/Core/Enemys/BP_NPC_Base` (`self.K2_GetPawn`)))
        (`/Game/XYZ_GD_Project/Core/Enemys/BP_NPC_Base.Refrash Agression Bar` _asbp_npc_base (`self.fAgression`) (`self.fAgressionAttaks`) (`self.fMaxAgression`))))))

(event `SetDamage`
  (params (fDamage :type "Float (double-precision)"))
  ;[1 0.4323 0.4323] SetDamage
  (if (`self.IsLife`)
    (bind _output_get (set `self.fHealt` (- (`self.fHealt`) fDamage)))
    (`self.Dransfer Data Heals BaseClass`)
    (`self.Damage Events` fDamage)
    (bind _returnvalue (`KismetSystemLibrary.K2_SetTimerDelegate` (delegate `dTimeStun`) 0.1 (> (`self.fStun`) 0.0)))
    (set `self.TimerStun` _returnvalue)
    (if (<= _output_get 0.0)
      (`KismetSystemLibrary.Delay` 0.5)
      (set `self.IsLife` false)
      (`self.Dransfer Data Life BaseClass`)
      (`KismetSystemLibrary.K2_ClearAndInvalidateTimerHandle` (`self.TimerDecreaseInAggression`))
      (`self.UnPossess`)
      (bind _asbp_player_character (cast `/Game/XYZ_GD_Project/Core/Character/BP_PlayerCharacter` (`GameplayStatics.GetPlayerCharacter` 0)))
      (`/Game/XYZ_GD_Project/Core/Character/BP_PlayerCharacter.SetPitchGame` _asbp_player_character true 0.002))))

(event `dTimeStun`
  (bind _fstun (`self.fStun`))
  ;[1 1 1] Stun
  (set `self.fStun` (- _fstun 0.1))
  (if (> _fstun 0.0)
    (bind _asbp_npc_base (cast `/Game/XYZ_GD_Project/Core/Enemys/BP_NPC_Base` (`self.K2_GetPawn`)))
    (`/Game/XYZ_GD_Project/Core/Enemys/BP_NPC_Base.SpeedDinamicCalculation` _asbp_npc_base (0.0 0.0 0.0) 0.0 true)
    (else
      (`KismetSystemLibrary.K2_ClearAndInvalidateTimerHandle` (`self.TimerStun`)))))

(fn `UserConstructionScript`)