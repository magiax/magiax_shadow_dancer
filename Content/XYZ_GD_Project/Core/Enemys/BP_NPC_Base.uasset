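; Base enemy NPC pawn that works with BP_AI_Controller_Base, forwarding damage to it and exposing setters for health and life state.
; Sighting the player updates the blackboard and starts a timer that builds controller aggression.
; It scales walk speed by target distance and shows a health/aggression widget when the player is near or on demand.
; Death disables collision, clears the weapon and, after a delay, emits gas whose particle collisions deal player-only radial damage.
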(event `self.ReceiveTick`
  (params (DeltaSeconds :type "Float (single-precision)"))
  (bind _healtui (`self.HealtUI`))
  (bind _fuishow (`self.fUIShow`))
  (set `self.fDeltaTime` DeltaSeconds)
  (if (`self.bIsLife`)
    (`|ExecutionSequence`
      (:`then_0`
        ;[0.9387 1 0.5512] Show LifeBar
        (if (> _fuishow 0.0)
          (set `self.fUIShow` (- (`self.fUIShow`) (`GameplayStatics.GetWorldDeltaSeconds`))))
        (if (or (< (`KismetMathLibrary.VSize` (- (`SceneComponent.K2_GetComponentLocation` (`self.Mesh`)) (`SceneComponent.K2_GetComponentLocation` (`Character.Mesh` (`GameplayStatics.GetPlayerCharacter` 0))))) 500.0) (> _fuishow 0.0))
          (`SceneComponent.SetVisibility` _healtui true false)
          (else
            (`SceneComponent.SetVisibility` _healtui false false))))
      (:`then_1`
        (bind _asumg_npc_life (cast `/Game/XYZ_GD_Project/UMG/UMG_NPC_Life` (`WidgetComponent.GetUserWidgetObject` (`self.HealtUI`))))
        (`/Game/XYZ_GD_Project/UMG/UMG_NPC_Life.RefrashLifeBar` _asumg_npc_life (`self.Healt`) (`self.MaxHealt`))))
    (else
      ;[1 1 1] Dead No Collision
      (`PrimitiveComponent.SetCollisionEnabled` (`self.Mesh`) "NoCollision")
      (`PrimitiveComponent.SetCollisionEnabled` (`self.CapsuleComponent`) "NoCollision")
      (`NavModifierComponent.SetAreaClass` (`self.NavModifier`) "/Script/NavigationSystem.NavArea_Default")
      (`ChildActorComponent.SetChildActorClass` (`self.BP_WeaponRight`) null)
      ;[1 1 1] Gas Generation
      (if (not (`self.bGasPosthumous`))
        (set `self.bGasPosthumous` true)
        (`KismetSystemLibrary.Delay` 10.0)
        (`self.GasPosthumous`)))))

(event `SetLife`
  (params (bLife :type Boolean))
  ;[1 1 1] Get/SetFromAIController
  (bind _output_get (set `self.bIsLife` bLife))
  (`self.HiddenUI` _output_get))

(event `SeesTarget`
  (params (bSees :type Boolean) (SeesActor :type "Actor Object Reference"))
  ;[1 0.3228 0.3328] AgressionUp
  (bind _output_get (set `self.bISeeTarget` bSees))
  (if _output_get
    (bind _returnvalue (`KismetSystemLibrary.K2_SetTimerDelegate` (delegate `AgressionUp`) 0.1 (`self.bISeeTarget`)))
    (set `self.TimerArgessive` _returnvalue)
    (else
      (`KismetSystemLibrary.K2_ClearAndInvalidateTimerHandle` (`self.TimerArgessive`)))))

(event `self.AIPerception.OnTargetPerceptionUpdated`
  (params (Actor :type "Actor Object Reference") (Stimulus :type "AIStimulus Structure"))
  (bind (_age _expirationage _strength _stimuluslocation _receiverlocation _tag _bsuccessfullysensed) (break `AIStimulus` Stimulus))
  ;[1 1 1] Enemy Sees Player
  (if (`self.bIsLife`)
    (if (`self.ActorHasTag` Actor "Player")
      (`self.SeesTarget` _bsuccessfullysensed Actor)
      (`BlackboardComponent.SetValueAsBool` (`AIBlueprintHelperLibrary.GetBlackboard` null) "bSeesTarget" _bsuccessfullysensed))))

(event `SetActualHealt`
  (params (fMaxHealt :type "Float (double-precision)") (fHealt :type "Float (double-precision)"))
  ;[1 1 1] Get/SetFromAIController
  (set `self.MaxHealt` fMaxHealt)
  (set `self.Healt` fHealt))

(event `AgressionUp`
  ;[1 0.3228 0.3328] AgressionUp
  (if (`self.ActorHasTag` (stale `SeesTarget` SeesActor) "Player")
    (bind _asbp_ai_controller_base (cast `/Game/XYZ_GD_Project/Core/Enemys/BaseAI/BP_AI_Controller_Base` (`self.GetOwner`)))
    (bind _asbp_player_character (cast `/Game/XYZ_GD_Project/Core/Character/BP_PlayerCharacter` (stale `SeesTarget` SeesActor)))
    (bind _fagression (`/Game/XYZ_GD_Project/Core/Enemys/BaseAI/BP_AI_Controller_Base.fAgression` _asbp_ai_controller_base))
    (if (< _fagression 50.0)
      (set `/Game/XYZ_GD_Project/Core/Enemys/BaseAI/BP_AI_Controller_Base.fAgression` (+ _fagression (`self.fSeesAgression`)) _asbp_ai_controller_base))
    (`BlackboardComponent.SetValueAsVector` (`AIBlueprintHelperLibrary.GetBlackboard` null) "vTargetPoint" (`SceneComponent.K2_GetComponentLocation` (`Character.Mesh` _asbp_player_character)))))

(event `SetShowUI`
  (params (fdTume :type "Float (double-precision)"))
  ;[1 1 1] Get/SetFromAIController
  (set `self.fUIShow` fdTume))

(event `Refrash Agression Bar`
  (params (fAgression :type "Float (double-precision)") (fAttackAgression :type "Float (double-precision)") (fMaxAgression :type "Float (double-precision)"))
  ;[1 1 1] Agression UI
  (bind _asumg_npc_life (cast `/Game/XYZ_GD_Project/UMG/UMG_NPC_Life` (`WidgetComponent.GetUserWidgetObject` (`self.HealtUI`))))
  (`/Game/XYZ_GD_Project/UMG/UMG_NPC_Life.RefrashAgression` _asumg_npc_life fAgression fAttackAgression fMaxAgression))

(event `SpeedDinamicCalculation`
  (params (vTargetPoint :type "Vector Structure") (fSpeed :type "Float (double-precision)") (ifFixed :type Boolean))
  ;[1 1 1] Dinamic Speed
  (if ifFixed
    (set `self.fSpeed` fSpeed)
    (set `CharacterMovementComponent.MaxWalkSpeed` (`self.fSpeed`) (`self.CharacterMovement`) :!label _label)
    (else
      (set `self.vTargetPoint` vTargetPoint)
      (`KismetSystemLibrary.K2_SetTimerDelegate` (delegate `SpeedCalculation`) 0.1 (> (`KismetMathLibrary.VSizeXY` (- (`self.vTargetPoint`) (`SceneComponent.K2_GetComponentLocation` (`self.Mesh`)))) 50.0)))))

(event `self.ReceiveAnyDamage`
  (params (Damage :type "Float (single-precision)") (DamageType :type "DamageType Object Reference") (InstigatedBy :type "Controller Object Reference") (DamageCauser :type "Actor Object Reference"))
  ;[1 1 1] Translite Damage
  (if (== (`GameplayStatics.GetObjectClass` DamageType) "/Game/XYZ_GD_Project/Weapons/BP_DamageAll.BP_DamageAll_C")
    (bind _asbp_ai_controller_base (cast `/Game/XYZ_GD_Project/Core/Enemys/BaseAI/BP_AI_Controller_Base` (`self.GetOwner`)))
    (`/Game/XYZ_GD_Project/Core/Enemys/BaseAI/BP_AI_Controller_Base.SetDamage` _asbp_ai_controller_base Damage)))

(event `SpeedCalculation`
  (bind _fmaxspeed (`self.fMaxSpeed`))
  (bind _returnvalue (`KismetMathLibrary.VSizeXY` (- (`self.vTargetPoint`) (`SceneComponent.K2_GetComponentLocation` (`self.Mesh`)))))
  ;[1 1 1] Dinamic Speed
  (if (> _returnvalue 1200.0)
    (set `self.fSpeed` _fmaxspeed)
    (goto _label)
    (else
      (set `self.fSpeed` (+ (`self.fMinSpeed`) (* _fmaxspeed (/ _returnvalue 1200.0))))
      (goto _label))))

(event `self.PS_Posthumous_head.OnParticleCollide`
  (params (EventName :type Name) (EmitterTime :type "Float (single-precision)") (ParticleTime :type Integer) (Location :type "Vector Structure") (Velocity :type "Vector Structure") (Direction :type "Vector Structure") (Normal :type "Vector Structure") (BoneName :type Name) (PhysMat :type "PhysicalMaterial Object Reference"))
  (bind _fgasdamage (`self.fGasDamage`))
  ;[0.1036 1 0.2361] Posthumous Damage Gas
  (`GameplayStatics.ApplyRadialDamageWithFalloff` :`BaseDamage` _fgasdamage :`MinimumDamage` _fgasdamage :`Origin` Location :`DamageInnerRadius` 1.0 :`DamageOuterRadius` 1.0 :`DamageFalloff` 2.0 :`DamageTypeClass` "/Game/XYZ_GD_Project/Weapons/BP_DamageOnlyPlayer.BP_DamageOnlyPlayer_C" :`DamageCauser` null :`InstigatedByController` null))

(event `self.PS_Posthumous_body_up.OnParticleCollide`
  (params (EventName :type Name) (EmitterTime :type "Float (single-precision)") (ParticleTime :type Integer) (Location :type "Vector Structure") (Velocity :type "Vector Structure") (Direction :type "Vector Structure") (Normal :type "Vector Structure") (BoneName :type Name) (PhysMat :type "PhysicalMaterial Object Reference"))
  (bind _fgasdamage (`self.fGasDamage`))
  ;[0.1036 1 0.2361] Posthumous Damage Gas
  (`GameplayStatics.ApplyRadialDamageWithFalloff` :`BaseDamage` _fgasdamage :`MinimumDamage` _fgasdamage :`Origin` Location :`DamageInnerRadius` 1.0 :`DamageOuterRadius` 1.0 :`DamageFalloff` 2.0 :`DamageTypeClass` "/Game/XYZ_GD_Project/Weapons/BP_DamageOnlyPlayer.BP_DamageOnlyPlayer_C" :`DamageCauser` null :`InstigatedByController` null))

(event `self.PS_Posthumous_body_down.OnParticleCollide`
  (params (EventName :type Name) (EmitterTime :type "Float (single-precision)") (ParticleTime :type Integer) (Location :type "Vector Structure") (Velocity :type "Vector Structure") (Direction :type "Vector Structure") (Normal :type "Vector Structure") (BoneName :type Name) (PhysMat :type "PhysicalMaterial Object Reference"))
  (bind _fgasdamage (`self.fGasDamage`))
  ;[0.1036 1 0.2361] Posthumous Damage Gas
  (`GameplayStatics.ApplyRadialDamageWithFalloff` :`BaseDamage` _fgasdamage :`MinimumDamage` _fgasdamage :`Origin` Location :`DamageInnerRadius` 1.0 :`DamageOuterRadius` 1.0 :`DamageFalloff` 2.0 :`DamageTypeClass` "/Game/XYZ_GD_Project/Weapons/BP_DamageOnlyPlayer.BP_DamageOnlyPlayer_C" :`DamageCauser` null :`InstigatedByController` null))

(fn `GetPatrolPoints`
  (returns (Points :type "Array of Vector Structure") (bIsPatrol :type Boolean))
  (bind _patrolpionts (`self.PatrolPionts`))
  (return _patrolpionts (> (`KismetArrayLibrary.Array_Length` _patrolpionts) 0)))

(fn `UserConstructionScript`)