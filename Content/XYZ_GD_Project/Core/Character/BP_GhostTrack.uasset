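; BP_GhostTrack is a ghost trail actor that leaves a fading afterimage of the player character's pose.
; On BeginPlay it copies the player's mesh pose onto GhostMesh and gives each material slot a dynamic MI_GhostTrack instance starting at zero opacity.
; GhostDestroy waits for a given delay, drives the opacity of those instances with a timeline, then destroys the actor.
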(event `self.ReceiveBeginPlay`
  ;[1 1 1] Start Ref
  (bind _asbp_player_character (cast `/Game/XYZ_GD_Project/Core/Character/BP_PlayerCharacter` (`GameplayStatics.GetPlayerPawn` 0)))
  (set `self.PlayerRef` _asbp_player_character)
  (`self.GhostTrails`))

(event `GhostTrails`
  ;[1 1 1] Creare Chost Trail Mesh
  (for _ (`MeshComponent.GetMaterials` (`self.GhostMesh`))
    (bind _returnvalue (`KismetMaterialLibrary.CreateDynamicMaterialInstance` "/Game/XYZ_GD_Project/Core/Character/Ghost/Mesh/MI_GhostTrack.MI_GhostTrack"))
    (bind _returnvalue_2 (`KismetArrayLibrary.Array_Add` (`self.DynamicMats`) _returnvalue))
    (`PrimitiveComponent.SetMaterial` (`self.GhostMesh`) _returnvalue_2 _returnvalue)
    (`MaterialInstanceDynamic.SetScalarParameterValue` _returnvalue "Opacity" 0.0)
    (`PoseableMeshComponent.CopyPoseFromSkeletalComponent` (`self.GhostMesh`) (`Character.Mesh` (`self.PlayerRef`)))))

(event `GhostDestroy`
  (params (Delay :type "Float (double-precision)"))
  ;[1 0.3854 0.3854] Destroy
  (`KismetSystemLibrary.Delay` Delay)
  (bind (_direction _newtrack_0) (`Timeline|TimelineVisible`)
    (:`Update`
      (for _array_element (`self.DynamicMats`)
        (`MaterialInstanceDynamic.SetScalarParameterValue` _array_element "Opacity" _newtrack_0)))
    (:`Finished`
      (`self.K2_DestroyActor` self))))

(fn `UserConstructionScript`)