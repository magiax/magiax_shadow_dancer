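; BP_Ghost is a posed ghost of the player that performs the selected weapon's action when spawned.
; It mirrors the weapon loadout, then reloads if empty, melees tagged enemies via line trace, or fires at markers chosen by side angle and distance.
; It copies player poses, rotating arm bones toward shot targets.
; A timer spawns BP_GhostTrack trail actors at the player until GhostDestroy clears them with staggered delays.
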(event `GhostTrails`
  (bind _playerref (`self.PlayerRef`))
  (bind _playerref_2 (`self.PlayerRef`))
  (bind _markers (`/Game/XYZ_GD_Project/Core/Character/BP_PlayerCharacter.Markers` _playerref))
  (bind _eplayerstateaction (`/Game/XYZ_GD_Project/Core/Character/BP_PlayerCharacter.ePlayerStateAction` _playerref_2))
  (bind _selectedweapon (`/Game/XYZ_GD_Project/Core/Character/BP_PlayerCharacter.SelectedWeapon` _playerref))
  ;[1 1 1] SelectWeapons
  (bind _reload (`self.WeaponsActionsBy` _playerref))
  (if _reload
    (set `/Game/XYZ_GD_Project/Core/Character/BP_PlayerCharacter.bShoot` false _playerref)
    ;[1 1 1] Reload Pose
    (if (or (`|EnumEquality` _eplayerstateaction "NewEnumerator0") (`|EnumEquality` _eplayerstateaction "NewEnumerator1") (`|EnumEquality` _eplayerstateaction "NewEnumerator4") (`|EnumEquality` _eplayerstateaction "NewEnumerator5"))
      (bind _sound_reload (`self.WeaponsActionsReload` _playerref))
      (`PoseableMeshComponent.CopyPoseFromSkeletalComponent` (`self.GhostMesh`) (`/Game/XYZ_GD_Project/Core/Character/BP_PlayerCharacter.InvisiablePoseFight` _playerref_2))
      (`GameplayStatics.PlaySound2D` _sound_reload 1.0 1.0 0.0 null null)
      (set `/Game/XYZ_GD_Project/Core/Character/BP_PlayerCharacter.fTimerTheDance` 0.0 (`self.PlayerRef`) :!label _label)
      (else
        ;[1 1 1] Copy Player Pawn Pose
        (`PoseableMeshComponent.CopyPoseFromSkeletalComponent` (`self.GhostMesh`) (`Character.Mesh` (`self.PlayerRef`)) :!label _label_2)))
    (else
      (switch `int` _selectedweapon
        (:`0`
          (bind (_outhit _attack) (`self.MeleeAttack` _playerref))
          (bind _output_get (set `/Game/XYZ_GD_Project/Core/Character/BP_PlayerCharacter.bShoot` _attack _playerref))
          (if _output_get
            ;[1 1 1] Melee Fight Pose
            (`PoseableMeshComponent.CopyPoseFromSkeletalComponent` (`self.GhostMesh`) (`/Game/XYZ_GD_Project/Core/Character/BP_PlayerCharacter.InvisiablePoseFight` (`self.PlayerRef`)))
            (`GameplayStatics.PlaySound2D` "/Game/XYZ_GD_Project/Audio/SwingOnImpact/SwingOnImpacts_Cue.SwingOnImpacts_Cue" 1.0 1.0 0.0 null null)
            (`self.MeleeDamage` _outhit)
            (goto _label)
            (else
              (goto _label_2))))
        (:`1`
          _)
        (:`2`
          _))
      (bind (_totalleftvector _totalrightvector _totalleftindex _totalrightindex) (`self.PointForShoting` _playerref (and (!= (`ChildActorComponent.ChildActorClass` (`self.BP_WeaponRight`)) null) (!= (`ChildActorComponent.ChildActorClass` (`self.BP_WeaponLeft`)) null)) _markers _selectedweapon))
      (bind _output_get_2 (set `/Game/XYZ_GD_Project/Core/Character/BP_PlayerCharacter.bShoot` (or (!= _totalleftindex -1) (!= _totalrightindex -1)) _playerref))
      (if _output_get_2
        ;[1 1 1] Range Pose
        (`PoseableMeshComponent.CopyPoseFromSkeletalComponent` (`self.GhostMesh`) (`Character.Mesh` (`self.PlayerRef`)))
        (`self.GenerationIgnoreArray` _playerref)
        (`self.Hand Positions Bone` _totalleftindex _totalrightindex _totalleftvector _totalrightvector _markers
          (:`Exit`
            (goto _label)))
        (else
          (goto _label_2)))))
  (`SceneComponent.SetVisibility` (`self.GhostMesh`) true false)
  ;[1 1 1] GeneratorTails
  (bind _returnvalue (`KismetSystemLibrary.K2_SetTimerDelegate` (delegate `ConstructTraseGhost`) 0.1 (not (`self.get/set Status`))))
  (set `self.Timer HandleTraseGhoste` _returnvalue))

(event `ConstructTraseGhost`
  ;[1 1 1] GeneratorTails
  (bind _returnvalue (`|SpawnActorFromClass` "/Game/XYZ_GD_Project/Core/Character/BP_GhostTrack.BP_GhostTrack_C" (`SceneComponent.K2_GetComponentToWorld` (`Character.Mesh` (`GameplayStatics.GetPlayerCharacter` 0))) "Undefined" "OverrideRootScale" null null))
  (`KismetArrayLibrary.Array_Add` (`self.GhoshTracks`) _returnvalue)
  (if (not (not (`self.get/set Status`)))
    (`KismetSystemLibrary.K2_ClearAndInvalidateTimerHandle` (`self.Timer HandleTraseGhoste`))))

(event `self.ReceiveBeginPlay`
  (bind _bp_weaponback (`self.BP_WeaponBack`))
  (bind _bp_weaponspin1left (`self.BP_WeaponSpin1Left`))
  (bind _bp_weaponleft (`self.BP_WeaponLeft`))
  (bind _bp_weaponright (`self.BP_WeaponRight`))
  (bind _bp_weaponspin1right (`self.BP_WeaponSpin1Right`))
  ;[0.4583 1 0.561] Construct
  (bind _asbp_player_character (cast `/Game/XYZ_GD_Project/Core/Character/BP_PlayerCharacter` (`GameplayStatics.GetPlayerPawn` 0)))
  (bind _output_get (set `self.PlayerRef` _asbp_player_character))
  (switch `int` (`/Game/XYZ_GD_Project/Core/Character/BP_PlayerCharacter.SelectedWeapon` _output_get)
    (:`0`
      (`ChildActorComponent.SetChildActorClass` _bp_weaponleft null)
      (`ChildActorComponent.SetChildActorClass` _bp_weaponright null)
      (`ChildActorComponent.SetChildActorClass` _bp_weaponback "/Game/XYZ_GD_Project/Weapons/BP_Shotgun.BP_Shotgun_C")
      (`ChildActorComponent.SetChildActorClass` _bp_weaponspin1left "/Game/XYZ_GD_Project/Weapons/BP_Pistol.BP_Pistol_C")
      (`ChildActorComponent.SetChildActorClass` _bp_weaponspin1right "/Game/XYZ_GD_Project/Weapons/BP_Pistol.BP_Pistol_C"))
    (:`1`
      (`ChildActorComponent.SetChildActorClass` _bp_weaponleft null)
      (`ChildActorComponent.SetChildActorClass` _bp_weaponright "/Game/XYZ_GD_Project/Weapons/BP_Shotgun.BP_Shotgun_C")
      (`ChildActorComponent.SetChildActorClass` _bp_weaponback null)
      (`ChildActorComponent.SetChildActorClass` _bp_weaponspin1left "/Game/XYZ_GD_Project/Weapons/BP_Pistol.BP_Pistol_C")
      (`ChildActorComponent.SetChildActorClass` _bp_weaponspin1right "/Game/XYZ_GD_Project/Weapons/BP_Pistol.BP_Pistol_C"))
    (:`2`
      (`ChildActorComponent.SetChildActorClass` _bp_weaponleft "/Game/XYZ_GD_Project/Weapons/BP_Pistol.BP_Pistol_C")
      (`ChildActorComponent.SetChildActorClass` _bp_weaponright "/Game/XYZ_GD_Project/Weapons/BP_Pistol.BP_Pistol_C")
      (`ChildActorComponent.SetChildActorClass` _bp_weaponback "/Game/XYZ_GD_Project/Weapons/BP_Shotgun.BP_Shotgun_C")
      (`ChildActorComponent.SetChildActorClass` _bp_weaponspin1left null)
      (`ChildActorComponent.SetChildActorClass` _bp_weaponspin1right null)))
  (`self.GhostTrails`))

(event `GhostDestroy`
  (bind _ghoshtracks (`self.GhoshTracks`))
  ;[0.224 0.07349 0.07349] Destroy
  (set `self.get/set Status` true)
  (`SceneComponent.SetVisibility` (`self.GhostMesh`) false true)
  (for (_array_element _array_index) _ghoshtracks
    (`/Game/XYZ_GD_Project/Core/Character/BP_GhostTrack.GhostDestroy` _array_element (* _array_index 0.001)))
  (`KismetArrayLibrary.Array_Clear` _ghoshtracks)
  (`KismetSystemLibrary.Delay` 0.2)
  (`self.K2_DestroyActor` self))

(fn `MeleeAttack`
  (params (`Player ref` :type "/Game/XYZ_GD_Project/Core/Character/BP_PlayerCharacter Object Reference"))
  (returns (OutHit :type "HitResult Structure") (Attack :type Boolean))
  (locals (LocalHit :type "HitResult Structure") (bAttack :type Boolean :default true))
  (bind (_outhit _returnvalue) (`KismetSystemLibrary.LineTraceSingleForObjects` (`SceneComponent.K2_GetComponentLocation` (`self.SocketHeadPhone`)) (`SceneComponent.K2_GetComponentLocation` (`self.SphereMelee`)) (`|MakeArray` "ObjectTypeQuery3" "ObjectTypeQuery2" :!type "EObjectTypeQuery Enum") false (`|MakeArray` (`self.PlayerRef`) :!type "Actor Object Reference") "None" true (struct :`R` 0.962642 :`G` 1.0 :`A` 1.0) (struct :`R` 0.032125 :`B` 1.0 :`A` 1.0)))
  (if (and _returnvalue (`|EnumEquality` (`/Game/XYZ_GD_Project/Core/Character/BP_PlayerCharacter.ePlayerStateAction` `Player ref`) "NewEnumerator0") true)
    (if (`self.ActorHasTag` (`.HitActor` (`GameplayStatics.BreakHitResult` _outhit)) "Enemy")
      (set `local.bAttack` true)
      (else
        (set `local.bAttack` false :!label _label)))
    (else
      (goto _label)))
  (return _outhit (`local.bAttack`)))

(fn `PointForShoting`
  (params (`Player ref` :type "/Game/XYZ_GD_Project/Core/Character/BP_PlayerCharacter Object Reference") (`Two guns` :type Boolean) (Markers :type "Array of /Game/XYZ_GD_Project/Core/Character/BP_Marker Object Reference") (Weapon :type Integer))
  (returns (TotalLeftVector :type "Vector Structure") (TotalRightVector :type "Vector Structure") (TotalLeftIndex :type Integer) (TotalRightIndex :type Integer))
  (locals (LeftVector :type "Vector Structure") (RightVector :type "Vector Structure") (iLeftIndex :type Integer :default -1) (iRightIndex :type Integer :default -1) (fReversLimitAngle :type "Float (double-precision)" :default -75.0) (fMaximumLimitAngle :type "Float (double-precision)" :default 120.0) (fMinLenghtGhot :type "Float (double-precision)"))
  (bind _fmaximumlimitangle (`local.fMaximumLimitAngle`))
  (bind _mesh (`Character.Mesh` `Player ref`))
  (bind _fangleshot (`self.fAngleShot`))
  (bind _returnvalue (`SceneComponent.K2_GetComponentLocation` _mesh))
  (bind (_returnvalue_roll _returnvalue_pitch _returnvalue_yaw) (`KismetMathLibrary.BreakRotator` (`SceneComponent.K2_GetComponentRotation` _mesh)))
  (bind _returnvalue_2 (* (`KismetMathLibrary.Conv_BoolToDouble` (not `Two guns`)) (`local.fReversLimitAngle`)))
  (switch `int` Weapon
    (:`Default`
      (set `local.fMinLenghtGhot` 170.0 :!label _label))
    (:`0`
      _)
    (:`1`
      (goto _label))
    (:`2`
      (set `local.fMinLenghtGhot` 150.0)))
  (for (_array_element _array_index) Markers
    (bind _returnvalue_location (`KismetMathLibrary.BreakTransform` (`self.GetTransform` _array_element)))
    (bind (_returnvalue_roll_2 _returnvalue_pitch_2 _returnvalue_yaw_2) (`KismetMathLibrary.BreakRotator` (`KismetMathLibrary.FindLookAtRotation` _returnvalue _returnvalue_location)))
    (bind _returnvalue_3 (- _returnvalue_yaw (- _returnvalue_yaw_2 90.0)))
    (if (> _returnvalue_3 180.0)
      (set `self.fAngleShot` (* -1 (- 360.0 _returnvalue_3)))
      (else
        (set `self.fAngleShot` _returnvalue_3)))
    (bind _returnvalue_4 (> (`KismetMathLibrary.VSize` (- _returnvalue_location _returnvalue)) (`local.fMinLenghtGhot`)))
    (if (and (>= _fangleshot _returnvalue_2) (< _fangleshot _fmaximumlimitangle) (== (`KismetMathLibrary.VSize` (`local.LeftVector`)) 0.0) _returnvalue_4)
      (set `local.LeftVector` _returnvalue_location)
      (set `local.iLeftIndex` _array_index))
    (if (and (> _fangleshot (* -1 _fmaximumlimitangle)) (< _fangleshot (* -1 _returnvalue_2)) (== (`KismetMathLibrary.VSize` (`local.RightVector`)) 0.0) _returnvalue_4)
      (set `local.RightVector` _returnvalue_location)
      (set `local.iRightIndex` _array_index)))
  (return (`local.LeftVector`) (`local.RightVector`) (`local.iLeftIndex`) (`local.iRightIndex`)))

(fn `UserConstructionScript`)

(fn `WeaponsActionsBy`
  (params (`Player ref` :type "/Game/XYZ_GD_Project/Core/Character/BP_PlayerCharacter Object Reference"))
  (returns (reload :type Boolean))
  (locals (WeaponReload :type Boolean))
  (bind _selectedweapon (`/Game/XYZ_GD_Project/Core/Character/BP_PlayerCharacter.SelectedWeapon` `Player ref`))
  (if (and (<= (`|GetArrayItem` (`/Game/XYZ_GD_Project/Core/Character/BP_PlayerCharacter.WeaponBullets` `Player ref`) _selectedweapon) 0) (!= _selectedweapon 0) true)
    (set `local.WeaponReload` true)
    (else
      (set `local.WeaponReload` false)))
  (return (`local.WeaponReload`)))

(fn `WeaponsActionsReload`
  (params (`Player ref` :type "/Game/XYZ_GD_Project/Core/Character/BP_PlayerCharacter Object Reference"))
  (returns (`Sound Reload` :type "SoundCue Object Reference"))
  (locals (WeaponReload :type Boolean))
  (bind _selectedweapon (`/Game/XYZ_GD_Project/Core/Character/BP_PlayerCharacter.SelectedWeapon` `Player ref`))
  (`KismetArrayLibrary.Array_Set` (`/Game/XYZ_GD_Project/Core/Character/BP_PlayerCharacter.WeaponBullets` `Player ref`) _selectedweapon (`|GetArrayItem` (`/Game/XYZ_GD_Project/Core/Character/BP_PlayerCharacter.WeaponBulletsMax` `Player ref`) _selectedweapon))
  (return (`|GetArrayItem` (`/Game/XYZ_GD_Project/Core/Character/BP_PlayerCharacter.WeaponReloadCue` `Player ref`) _selectedweapon)))