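; BP_Marker is a marker actor that follows an assigned carrier actor around the world.
; Magnetic stores the carrier and starts a looping 0.1-second timer that snaps the Marker component to the carrier's root location, avoiding Tick.
; GestroyMarker clears that timer if its handle is valid, then destroys the actor.
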(event `Magnetic`
  (params (Carrier :type "Actor Object Reference"))
  (set `self.RefCarrier` Carrier)
  (bind _returnvalue (`KismetSystemLibrary.K2_SetTimerDelegate` (delegate `ReLocationPawn`) 0.1 true))
  (set `self.TimerReLocation` _returnvalue))

(event `ReLocationPawn`
  (`SceneComponent.K2_SetWorldLocation` (`self.Marker`) (`SceneComponent.K2_GetComponentLocation` (`Actor.RootComponent` (`self.RefCarrier`))) false false))

(fn `Gestroy Marker`
  (bind _timerrelocation (`self.TimerReLocation`))
  (if (`KismetSystemLibrary.K2_IsValidTimerHandle` _timerrelocation)
    (`KismetSystemLibrary.K2_ClearAndInvalidateTimerHandle` _timerrelocation))
  (`self.K2_DestroyActor`))

(fn `UserConstructionScript`)