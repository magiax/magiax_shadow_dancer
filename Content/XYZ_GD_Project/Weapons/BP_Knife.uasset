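; BP_Knife is a melee knife weapon that deals damage when it overlaps an actor tagged Player.
; On overlap it applies small-radius radial damage at its Scene component using BP_DamageAll, with base and minimum damage both set to FDamage.
; The knife's parent actor is ignored, so a wielder holding it as a child actor is spared.
; BeginPlay, Tick and construction only call the parent class.
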(event `self.ReceiveBeginPlay`
  (`parent.ReceiveBeginPlay`))

(event `self.ReceiveTick`
  (params (DeltaSeconds :type "Float (single-precision)"))
  (`parent.ReceiveTick` DeltaSeconds))

(event `self.ReceiveActorBeginOverlap`
  (params (OtherActor :type "Actor Object Reference"))
  (bind _fdamage (`self.fDamage`))
  (bind _scene (`self.Scene`))
  (if (`self.ActorHasTag` OtherActor "Player")
    (`GameplayStatics.ApplyRadialDamageWithFalloff` _fdamage _fdamage (`SceneComponent.K2_GetComponentLocation` _scene) 0.0 20.0 0.0 "/Game/XYZ_GD_Project/Weapons/BP_DamageAll.BP_DamageAll_C" (`|MakeArray` (`self.GetParentActor` (`ActorComponent.GetOwner` _scene))) self null)))

(fn `UserConstructionScript`
  (`parent.UserConstructionScript`))