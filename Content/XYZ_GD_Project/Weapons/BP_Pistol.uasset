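; BP_Pistol is a pistol weapon Blueprint that builds on a parent weapon class.
; On ShotWeapons it plays the gun's fire animation and a 2D fire sound.
; It then calls ShotAndTraceBullets from the Source component toward the given target, passing pellet count, per-pellet damage, scatter, min and max range, and an ignore list.
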(event `self.ShotWeapons`
  (params (Target :type "Vector Structure") (IgnorList :type "Array of Actor Object Reference (by ref)"))
  (`SkeletalMeshComponent.PlayAnimation` (`self.Gun`) "/Game/XYZ_GD_Project/Weapons/Pistols/Fire_Pistol_W.Fire_Pistol_W" false)
  (`GameplayStatics.PlaySound2D` "/Game/XYZ_GD_Project/Weapons/Sounds/Pistol/Cues/PistolA_Fire_Cue.PistolA_Fire_Cue" 1.0 1.0 0.0 null null)
  (`self.ShotAndTraceBullets` (`self.iPellets`) (`self.fDamageOnePellets`) (`self.fScatter`) (`self.fRangeMax`) (`self.fRangeMin`) (`SceneComponent.K2_GetComponentLocation` (`self.Source`)) Target IgnorList))

(event `self.ReceiveBeginPlay`
  (`parent.ReceiveBeginPlay`))

(fn `UserConstructionScript`
  (`parent.UserConstructionScript`))