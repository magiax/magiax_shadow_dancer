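; Base weapon Blueprint with an empty ShotWeapons event and a shared hitscan firing function, ShotAndTraceBullets.
; The function fires one line trace per pellet, randomized within a scatter cone and range band.
; Each hit spawns a Niagara tracer to the impact point and a BP_Hit actor given the damage, hit actor and whether the component is tagged Shield.
; Misses produce no tracer or hit actor.
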(event `self.ReceiveTick`
  (params (DeltaSeconds :type "Float (single-precision)")))

(event `ShotWeapons`
  (params (Target :type "Vector Structure") (IgnorList :type "Array of Actor Object Reference")))

(fn `ShotAndTraceBullets`
  (params (Pellets :type Integer) (Damage :type "Float (double-precision)") (Scatter :type "Float (double-precision)") (RangeMax :type "Float (double-precision)") (RangeMin :type "Float (double-precision)") (Start :type "Vector Structure") (End :type "Vector Structure") (IgnerList :type "Array of Actor Object Reference"))
  (for _ (range 1 (+ Pellets 1))
    (bind (_outhit _returnvalue) (`KismetSystemLibrary.LineTraceSingleForObjects` Start (+ Start (* (`KismetMathLibrary.RandomUnitVectorInConeInRadians` (- End Start) (`KismetMathLibrary.DegreesToRadians` Scatter)) (`KismetMathLibrary.RandomFloatInRange` RangeMin RangeMax))) (`|MakeArray` "ObjectTypeQuery1" "ObjectTypeQuery2" "ObjectTypeQuery4" "ObjectTypeQuery3" :!type "EObjectTypeQuery Enum") false IgnerList "None" true (struct :`R` 1.0 :`G` 0.00718 :`A` 1.0) (struct :`R` 0.744792 :`G` 0.643933 :`A` 1.0) 2.0))
    (if _returnvalue
      (bind (_bblockinghit _binitialoverlap _time _distance _location _impactpoint _normal _impactnormal _physmat _hitactor _hitcomponent _hitbonename _hititem _faceindex _tracestart) (`GameplayStatics.BreakHitResult` _outhit))
      (bind _returnvalue_2 (`NiagaraFunctionLibrary.SpawnSystemAtLocation` "/Game/XYZ_GD_Project/Weapons/ParticleSystem/Materials/NS_Bullet_Trace_System.NS_Bullet_Trace_System" _tracestart))
      (`FXSystemComponent.SetVectorParameter` _returnvalue_2 "EndPoint" _location)
      (bind _returnvalue_3 (`|SpawnActorFromClass` "/Game/XYZ_GD_Project/Weapons/Hit/BP_Hit.BP_Hit_C" (`KismetMathLibrary.MakeTransform` _location (`KismetMathLibrary.RandomRotator` true) (0.5 0.5 0.5)) "Undefined" "OverrideRootScale" null null))
      (`/Game/XYZ_GD_Project/Weapons/Hit/BP_Hit.SetParams` _returnvalue_3 Damage _hitactor (`ActorComponent.ComponentHasTag` _hitcomponent "Shield")))))

(fn `UserConstructionScript`)