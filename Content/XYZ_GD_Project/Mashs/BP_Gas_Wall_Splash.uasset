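; BP_Gas_Wall_Splash is a gas hazard that damages the player while they stand inside it.
; Activation turns on the gas particle trails and the Sphere; BeginPlay switches both off if not already active.
; A tagged player overlapping the active Sphere starts a fast looping timer that applies radial falloff damage around the Sphere through a player-only damage type.
; Ending the overlap clears the timer.
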(event `Activation`
  ;[1 1 1] Activation
  (set `self.bIsActive` true)
  (`ParticleSystemComponent.BeginTrails` (`self.Gas`) "None" "None" "ETrailWidthMode_FromCentre" 0.0)
  (`ActorComponent.SetActive` (`self.Sphere`) true true))

(event `self.ReceiveBeginPlay`
  ;[1 1 1] Begin
  (if (not (`self.bIsActive`))
    (`ParticleSystemComponent.EndTrails` (`self.Gas`))
    (`ActorComponent.SetActive` (`self.Sphere`) false false)))

(event `self.Sphere.OnComponentBeginOverlap`
  (params (OverlappedComponent :type "PrimitiveComponent Object Reference") (OtherActor :type "Actor Object Reference") (OtherComp :type "PrimitiveComponent Object Reference") (OtherBodyIndex :type Integer) (bFromSweep :type Boolean) (SweepResult :type "HitResult Structure (by ref)"))
  (bind _returnvalue (`self.ActorHasTag` OtherActor "Player"))
  (if (and (`self.bIsActive`) _returnvalue true)
    (set `self.bDamager` _returnvalue)
    (bind _returnvalue_2 (`KismetSystemLibrary.K2_SetTimerDelegate` (delegate `Damager`) 0.1 (`self.bDamager`)))
    (set `self.Timer` _returnvalue_2)))

(event `Damager`
  (bind _fgasdamage (`self.fGasDamage`))
  (`GameplayStatics.ApplyRadialDamageWithFalloff` :`BaseDamage` _fgasdamage :`MinimumDamage` _fgasdamage :`Origin` (`SceneComponent.K2_GetComponentLocation` (`self.Sphere`)) :`DamageOuterRadius` 300.0 :`DamageFalloff` 2.0 :`DamageTypeClass` "/Game/XYZ_GD_Project/Weapons/BP_DamageOnlyPlayer.BP_DamageOnlyPlayer_C" :`DamageCauser` null :`InstigatedByController` null))

(event `self.Sphere.OnComponentEndOverlap`
  (params (OverlappedComponent :type "PrimitiveComponent Object Reference") (OtherActor :type "Actor Object Reference") (OtherComp :type "PrimitiveComponent Object Reference") (OtherBodyIndex :type Integer))
  (if (`self.ActorHasTag` OtherActor "Player")
    (set `self.bDamager` false)
    (`KismetSystemLibrary.K2_ClearAndInvalidateTimerHandle` (`self.Timer`))))

(fn `UserConstructionScript`)