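; Shootable letter target pawn that is switched on with a type and takes hits until it is knocked out.
; ActiveLetter passes the type to the UMG_Info_Tarret widget on the Weapon component and sets hit points, with type 0 tougher than the rest.
; While active, each damage event removes one hit point regardless of amount.
; At zero it deactivates the widget, hides itself and disables Cube collision; GetActive exposes its state.
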(event `ActiveLetter`
  (params (iType :type Integer))
  (bind _asumg_info_tarret (cast `/Game/XYZ_GD_Project/UMG/UMG_Info_Tarret` (`WidgetComponent.GetUserWidgetObject` (`self.Weapon`))))
  (`/Game/XYZ_GD_Project/UMG/UMG_Info_Tarret.WeaponActive` _asumg_info_tarret iType)
  (set `self.bActiveTarget` true)
  (switch `int` iType
    (:`Default`
      (set `self.iLife` 1 :!label _label))
    (:`0`
      (set `self.iLife` 2))
    (:`1`
      (goto _label))
    (:`2`
      (goto _label))))

(event `self.ReceiveAnyDamage`
  (params (Damage :type "Float (single-precision)") (DamageType :type "DamageType Object Reference") (InstigatedBy :type "Controller Object Reference") (DamageCauser :type "Actor Object Reference"))
  (if (`self.bActiveTarget`)
    (bind _output_get (set `self.iLife` (- (`self.iLife`) 1)))
    (if (== _output_get 0)
      (bind _asumg_info_tarret (cast `/Game/XYZ_GD_Project/UMG/UMG_Info_Tarret` (`WidgetComponent.GetUserWidgetObject` (`self.Weapon`))))
      (`/Game/XYZ_GD_Project/UMG/UMG_Info_Tarret.WeaponDeactive` _asumg_info_tarret)
      (set `self.bActiveTarget` false)
      (`SceneComponent.SetVisibility` (`self.DefaultSceneRoot`) false true)
      (`PrimitiveComponent.SetCollisionEnabled` (`self.Cube`) "NoCollision"))))

(fn `getActive`
  (returns (bActive :type Boolean))
  (return (`self.bActiveTarget`)))

(fn `UserConstructionScript`)