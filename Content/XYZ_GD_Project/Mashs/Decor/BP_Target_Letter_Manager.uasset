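; BP_Target_Letter_Manager runs a scripted combat tutorial at a target range, teaching the player's colored forms, attacks and controls.
; When the player enters its Sphere, a looping timer polls active targets, removes inactive ones and starts the next wave once none remain.
; Each wave activates lettered targets, switches the player's tutorial music and sets toolbar instructions in Russian.
; The last step stops the timer and introduces the poison-gas section.
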(event `self.ReceiveBeginPlay`
  (bind _asbp_player_character (cast `/Game/XYZ_GD_Project/Core/Character/BP_PlayerCharacter` (`GameplayStatics.GetPlayerCharacter` 0)))
  (set `self.RefCharacter` _asbp_player_character))

(event `ScanTarget`
  (bind _arrayactive (`self.arrayActive`))
  (if (> (`KismetArrayLibrary.Array_Length` _arrayactive) 0)
    (for (_array_element _array_index) _arrayactive
      (if (not (`/Game/XYZ_GD_Project/Mashs/Decor/BP_Target_Letter_Pawn.bActiveTarget` _array_element))
        (`KismetArrayLibrary.Array_Remove` _arrayactive _array_index)))
    (else
      (`self.NextWave`))))

(event `self.Sphere.OnComponentBeginOverlap`
  (params (OverlappedComponent :type "PrimitiveComponent Object Reference") (OtherActor :type "Actor Object Reference") (OtherComp :type "PrimitiveComponent Object Reference") (OtherBodyIndex :type Integer) (bFromSweep :type Boolean) (SweepResult :type "HitResult Structure (by ref)"))
  (if (and (`self.ActorHasTag` OtherActor "Player") (not (`self.bIsStarted`)))
    (set `self.bIsStarted` true)
    (bind _returnvalue (`KismetSystemLibrary.K2_SetTimerDelegate` (delegate `ScanTarget`) 0.1 true))
    (set `self.Timer` _returnvalue)))

(event `NextWave`
  (bind _output (`|GetArrayItem` (`self.Targets`)))
  (bind _output_2 (`|GetArrayItem` (`self.Targets`) 2))
  (bind _output_3 (`|GetArrayItem` (`self.Targets`) 6))
  (bind _output_4 (`|GetArrayItem` (`self.Targets`) 3))
  (bind _output_5 (`|GetArrayItem` (`self.Targets`) 7))
  (bind _output_6 (`|GetArrayItem` (`self.Targets`) 5))
  (bind _output_7 (`|GetArrayItem` (`self.Targets`) 4))
  (bind _output_8 (`|GetArrayItem` (`self.Targets`) 1))
  (bind _umgtoolbarref (`/Game/XYZ_GD_Project/Core/Character/BP_PlayerCharacter.UMGToolbarRef` (`self.RefCharacter`)))
  (bind _asbp_player_character (cast `/Game/XYZ_GD_Project/Core/Character/BP_PlayerCharacter` (`GameplayStatics.GetPlayerCharacter` 0)))
  (`/Game/XYZ_GD_Project/Core/Character/BP_PlayerCharacter.StopPlayTitorialMusic` _asbp_player_character)
  (bind _output_get (set `self.iIndexActive` (+ (`self.iIndexActive`) 1)))
  (switch `int` _output_get
    (:`0`
      (`/Game/XYZ_GD_Project/Mashs/Decor/BP_Target_Letter_Pawn.ActiveLetter` _output 0)
      (`KismetArrayLibrary.Array_Add` (`self.arrayActive`) _output)
      (`/Game/XYZ_GD_Project/Core/Character/BP_PlayerCharacter.StartPlayTutorialMusic` _asbp_player_character 0)
      (`/Game/XYZ_GD_Project/UMG/UMG_Toolsbar.SetTextInformation` _umgtoolbarref "Для эффективного ближнего боя.  \nВыбери красную форму тела цифра \"1\"  \nи подойди лицом к мишени над которой светиться красный кулак."))
    (:`1`
      (`/Game/XYZ_GD_Project/Mashs/Decor/BP_Target_Letter_Pawn.ActiveLetter` _output_8 0)
      (`KismetArrayLibrary.Array_Add` (`self.arrayActive`) _output_8)
      (`/Game/XYZ_GD_Project/Core/Character/BP_PlayerCharacter.StartPlayTutorialMusic` _asbp_player_character 0)
      (`/Game/XYZ_GD_Project/UMG/UMG_Toolsbar.SetTextInformation` _umgtoolbarref "Атакуй следующую мишень с меткой.  \nДля ближней атаки не нужно нажимать никаких кнопок,  \nнужно лишь, что бы враг был перед тобой,  \nты был в красной форме и шли красные волны ритма."))
    (:`2`
      (`/Game/XYZ_GD_Project/Mashs/Decor/BP_Target_Letter_Pawn.ActiveLetter` _output_2 1)
      (`KismetArrayLibrary.Array_Add` (`self.arrayActive`) _output_2)
      (`/Game/XYZ_GD_Project/Core/Character/BP_PlayerCharacter.StartPlayTutorialMusic` _asbp_player_character 1)
      (`/Game/XYZ_GD_Project/UMG/UMG_Toolsbar.SetTextInformation` _umgtoolbarref "Выбери желтую форму, кнопка “2” прицелься  \nна мишень с символом дробовика и нажми ЛКМ.  \nЛевая Кнопка Мышки – ставит маркеры круглые на объекты."))
    (:`3`
      (`/Game/XYZ_GD_Project/Mashs/Decor/BP_Target_Letter_Pawn.ActiveLetter` _output_4 2)
      (`KismetArrayLibrary.Array_Add` (`self.arrayActive`) _output_4)
      (`/Game/XYZ_GD_Project/Mashs/Decor/BP_Target_Letter_Pawn.ActiveLetter` _output_7 2)
      (`KismetArrayLibrary.Array_Add` (`self.arrayActive`) _output_7)
      (`/Game/XYZ_GD_Project/Core/Character/BP_PlayerCharacter.StartPlayTutorialMusic` _asbp_player_character 2)
      (`/Game/XYZ_GD_Project/UMG/UMG_Toolsbar.SetTextInformation` _umgtoolbarref "Теперь выбери зеленую форму, кнопка “3”.  \nНажми ЛКМ на мишенях с знаком пистолетов.  \nЛюбая атака героя в игре происходит только,  \nкогда волна такого же цвета, как и герой – подходит к прицелу. \nПерезарядка происходит автоматически, когда заканчиваются патроны."))
    (:`4`
      (`/Game/XYZ_GD_Project/Mashs/Decor/BP_Target_Letter_Pawn.ActiveLetter` _output_6 2)
      (`KismetArrayLibrary.Array_Add` (`self.arrayActive`) _output_6)
      (`/Game/XYZ_GD_Project/Mashs/Decor/BP_Target_Letter_Pawn.ActiveLetter` _output_3 2)
      (`KismetArrayLibrary.Array_Add` (`self.arrayActive`) _output_3)
      (`/Game/XYZ_GD_Project/Core/Character/BP_PlayerCharacter.StartPlayTutorialMusic` _asbp_player_character 2)
      (`/Game/XYZ_GD_Project/UMG/UMG_Toolsbar.SetTextInformation` _umgtoolbarref "Дробовик хорош на средней дистанции, так как имеет разброс.  \nПистолеты удобны на средней и длинной дистанциях.  \nТак же пистолеты могу одновременно стрелять по 2 разным целям,  \nкоторые находятся по разные стороны от героя."))
    (:`5`
      (`/Game/XYZ_GD_Project/Mashs/Decor/BP_Target_Letter_Pawn.ActiveLetter` _output_5 1)
      (`KismetArrayLibrary.Array_Add` (`self.arrayActive`) _output_5)
      (`/Game/XYZ_GD_Project/Core/Character/BP_PlayerCharacter.StartPlayTutorialMusic` _asbp_player_character 1)
      (`/Game/XYZ_GD_Project/UMG/UMG_Toolsbar.SetTextInformation` _umgtoolbarref "Метки исезают примерно через 5-10 секунд, в зависимости от их востребованности. \nТак же для удобства стрельбы при отступлении можно переключиться в оборонительную стойку кнопкой “X”. Переключение обратно происходит нажатием той кнопки “X”. \n"))
    (:`6`
      (`KismetSystemLibrary.K2_ClearAndInvalidateTimerHandle` (`self.Timer`))
      (`/Game/XYZ_GD_Project/UMG/UMG_Toolsbar.SetTextInformation` _umgtoolbarref "Далее идёт секция с ядовитым газом.  \nГаз отнимает здоровье.  \nДля перекаты нажимай “Ctrl”. \nДля ускорения нажимай “Shift”. \nВ правом верхнем иглу - индикатор жизней."))))

(fn `UserConstructionScript`)