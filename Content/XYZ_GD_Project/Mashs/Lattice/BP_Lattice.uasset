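; Lattice (grate) hazard that vents selectable gas particle effects with matching sound, harming the player on contact.
; In automatic mode a looping timer fires waves only while the player is within sound range; BeginWaveGas triggers one at any distance.
; SetVolumeSound scales volume by horizontal distance to the player and reports whether it is audible.
; Particle collisions apply small-radius damage using a player-only damage type.
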(event `self.ReceiveBeginPlay`
  ;[1 1 1] Automatic Wave Gas
  (if (`self.bAutomatiks`)
    (`ParticleSystemComponent.SetTemplate` (`self.PS_Gas`) (`|GetArrayItem` (`self.PS_All_Gas`) (`self.iSelectGas`)))
    (bind _returnvalue (`KismetSystemLibrary.K2_SetTimerDelegate` (delegate `LaunchtGas`) (`self.fTimerRefrash`) true (`self.fDeltaStart`)))
    (set `self.Timer Wave` _returnvalue)))

(event `LaunchtGas`
  (bind _gas (`self.Gas`))
  ;[1 1 1] Automatic Wave Gas
  (bind _bactive (`self.SetVolumeSound`))
  (if _bactive
    (`ParticleSystemComponent.BeginTrails` (`self.PS_Gas`) "None" "None" "ETrailWidthMode_FromCentre" 0.0)
    (`AudioComponent.SetSound` _gas (`|GetArrayItem` (`self.AudioGas`) (`self.iSelectGas`)))
    (`AudioComponent.Play` _gas 0.0)))

(event `self.PS_Gas.OnParticleCollide`
  (params (EventName :type Name) (EmitterTime :type "Float (single-precision)") (ParticleTime :type Integer) (Location :type "Vector Structure") (Velocity :type "Vector Structure") (Direction :type "Vector Structure") (Normal :type "Vector Structure") (BoneName :type Name) (PhysMat :type "PhysicalMaterial Object Reference"))
  (bind _fdamage (`self.fDamage`))
  ;[0.1277 1 0.2754] Damage Gas
  (`GameplayStatics.ApplyRadialDamageWithFalloff` :`BaseDamage` _fdamage :`MinimumDamage` _fdamage :`Origin` Location :`DamageInnerRadius` 1.0 :`DamageOuterRadius` 1.0 :`DamageFalloff` 2.0 :`DamageTypeClass` "/Game/XYZ_GD_Project/Weapons/BP_DamageOnlyPlayer.BP_DamageOnlyPlayer_C" :`DamageCauser` null :`InstigatedByController` null))

(event `BeginWaveGas`
  (params (iSelectGas :type Integer))
  (bind _gas (`self.Gas`))
  (bind _ps_gas (`self.PS_Gas`))
  ;[1 0.877 0.3953] Begin Wave Gas
  (`ParticleSystemComponent.SetTemplate` _ps_gas (`|GetArrayItem` (`self.PS_All_Gas`) iSelectGas))
  (`ParticleSystemComponent.BeginTrails` _ps_gas "None" "None" "ETrailWidthMode_FromCentre" 0.0)
  (`self.SetVolumeSound`)
  (`AudioComponent.SetSound` _gas (`|GetArrayItem` (`self.AudioGas`) iSelectGas))
  (`AudioComponent.Play` _gas 0.0))

(fn `UserConstructionScript`)