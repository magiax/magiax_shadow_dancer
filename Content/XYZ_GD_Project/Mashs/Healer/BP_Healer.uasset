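; Healer pickup that calls SetHealer on the player character when a Player-tagged actor overlaps its mesh.
; A Life flag makes it single-use: it plays a sound, triggers the effect, then destroys itself after a short delay.
; On Tick, the mesh tumbles with a decaying speed, drawing a new random speed and rotation vector whenever it slows below a threshold.
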(event `self.ReceiveTick`
  (params (DeltaSeconds :type "Float (single-precision)"))
  (bind _staticmesh (`self.StaticMesh`))
  (bind (_returnvalue_roll _returnvalue_pitch _returnvalue_yaw) (`KismetMathLibrary.BreakRotator` (`SceneComponent.K2_GetComponentRotation` _staticmesh)))
  (bind (_returnvalue_x _returnvalue_y _returnvalue_z) (`KismetMathLibrary.BreakVector` (* (`self.vRotation`) (`self.fSpeed`))))
  (if (>= (`self.fSpeed`) 0.5)
    (bind _output_get (set `self.fSpeed` (/ (`self.fSpeed`) 1.01)))
    (bind _returnvalue (* _output_get 0.5))
    (`SceneComponent.K2_SetWorldRotation` _staticmesh (`KismetMathLibrary.MakeRotator` (+ _returnvalue_roll (* _returnvalue _returnvalue_x)) (+ _returnvalue_pitch (* _returnvalue _returnvalue_y)) (+ _returnvalue_yaw (* _returnvalue _returnvalue_z))) false false)
    (else
      (set `self.fSpeed` (`KismetMathLibrary.RandomFloatInRange` 1.0 1.3))
      (set `self.vRotation` (`KismetMathLibrary.MakeVector` (`KismetMathLibrary.RandomFloatInRange` -10.0 10.0) (`KismetMathLibrary.RandomFloatInRange` -10.0 10.0) (`KismetMathLibrary.RandomFloatInRange` -10.0 10.0))))))

(event `self.StaticMesh.OnComponentBeginOverlap`
  (params (OverlappedComponent :type "PrimitiveComponent Object Reference") (OtherActor :type "Actor Object Reference") (OtherComp :type "PrimitiveComponent Object Reference") (OtherBodyIndex :type Integer) (bFromSweep :type Boolean) (SweepResult :type "HitResult Structure (by ref)"))
  (if (and (`ActorComponent.ComponentHasTag` (`Actor.RootComponent` OtherActor) "Player") (`self.bLife`) true)
    (`AudioComponent.Play` (`self.SounEffect`) 0.0)
    (bind _asbp_player_character (cast `/Game/XYZ_GD_Project/Core/Character/BP_PlayerCharacter` (`GameplayStatics.GetPlayerCharacter` 0)))
    (`/Game/XYZ_GD_Project/Core/Character/BP_PlayerCharacter.SetHealer` _asbp_player_character)
    (set `self.bLife` false)
    (`KismetSystemLibrary.Delay` 0.7)
    (`self.K2_DestroyActor`)))

(fn `UserConstructionScript`)