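; BP_Car_Blocked_Boss is a car in the boss set that slides along a fixed path when activated, with sound playing during the move.
; Activation starts SoundMusic and a fast timer, which loops if the distance is within its maximum.
; Each CarMovie tick advances the car's relative X and lowers Z proportionally, using teleport moves.
; Once the distance exceeds the maximum, it clears the timer and stops the sound.
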(event `Activation`
  (bind _returnvalue (`KismetSystemLibrary.K2_SetTimerDelegate` (delegate `Car Movie`) 0.02 (<= (`self.fDistance`) (`self.fMaxDistance`))))
  (set `self.Timer` _returnvalue)
  (`AudioComponent.Play` (`self.SoundMusic`) 0.0))

(event `Car Movie`
  (bind _fdistance (`self.fDistance`))
  (if (<= (`self.fDistance`) (`self.fMaxDistance`))
    (set `self.fDistance` (+ (`self.fDistance`) 10.0))
    (`SceneComponent.K2_SetRelativeLocation` (`self.Car`) (`KismetMathLibrary.MakeVector` _fdistance 0.0 (/ _fdistance -16.66667)) false true)
    (else
      (`KismetSystemLibrary.K2_ClearAndInvalidateTimerHandle` (`self.Timer`))
      (`AudioComponent.Stop` (`self.SoundMusic`)))))

(fn `UserConstructionScript`)